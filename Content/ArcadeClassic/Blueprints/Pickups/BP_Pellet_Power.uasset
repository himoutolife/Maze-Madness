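; BP_Pellet_Power is the power pellet pickup that makes enemies vulnerable when the player eats it.
; Player overlap with the mesh plays sound and eaten VFX, removes the mesh and glow, then destroys the actor after a delay.
; The same overlap reports the pellet to the gameplay game mode, notifies every enemy actor and adds points through the game instance.
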(event OnComponentBeginOverlap(SM_Power_Pellet)
  (params (OverlappedComponent :type Primitive%20Component%20Object%20Reference) (OtherActor :type Actor%20Object%20Reference) (OtherComp :type Primitive%20Component%20Object%20Reference) (OtherBodyIndex :type Integer) (bFromSweep :type Boolean) (SweepResult :type Hit%20Result%20Structure%20%28by%20ref%29))
  (Utilities|Casting|CastToBP_Player OtherActor)
  (Utilities|FlowControl|Sequence
    (:then_0
      ;[1 1 1] Power Pellet eaten handling
      (Audio|PlaySound2D "/Game/ArcadeClassic/Audio/SFX_EatSpecial_Cue.SFX_EatSpecial_Cue" 1.0 1.0 0.0 0 0)
      (Components|Activation|Activate (Variables|Default|GetVFX_Power_Pellet_Eaten) false)
      (Components|DestroyComponent (Variables|Default|GetSM_Power_Pellet))
      (Utilities|FlowControl|Delay 5.0)
      (Actor|DestroyActor))
    (:then_1
      ;[1 1 1] Game Mode BP- Decrement Level's pellet count
      (bind _asbp_game_mode_gameplay (Utilities|Casting|CastToBP_GameMode_Gameplay (Game|GetGameMode)))
      (Default|AtePellet _asbp_game_mode_gameplay))
    (:then_2
      ;[1 1 1] enemies to be vulnerable
      (bind _outactors (Actor|GetAllActorsOfClass "/Game/ArcadeClassic/Blueprints/Characters/BP_Enemy_parent.BP_Enemy_parent_C"))
      (Default|PowerPelletEaten _outactors))
    (:then_3
      ;[1 1 1] increments score
      (bind _asbp_game_instance (Utilities|Casting|CastToBP_GameInstance (Game|GetGameInstance)))
      (Default|AddPoints _asbp_game_instance (Variables|Default|GetPowerPelletPoints)))))

(fn ConstructionScript)