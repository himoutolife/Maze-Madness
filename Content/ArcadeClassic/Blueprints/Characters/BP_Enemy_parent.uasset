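; Parent Blueprint for Pac-Man-style maze enemies that either wander between random TargetPoints or hunt the player.
; A Tick-fed gate, opened by start/restart timers and closed on death, drives AI MoveTo navigation.
; Power pellets force wandering and run a timeline swapping vulnerable meshes.
; Player overlap either awards escalating points and respawns the enemy at its start, or kills the player and sends all enemies home.
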(event OnComponentBeginOverlap(Player_collision)
  (params (OverlappedComponent :type Primitive%20Component%20Object%20Reference) (OtherActor :type Actor%20Object%20Reference) (OtherComp :type Primitive%20Component%20Object%20Reference) (OtherBodyIndex :type Integer) (bFromSweep :type Boolean) (SweepResult :type Hit%20Result%20Structure%20%28by%20ref%29))
  (bind _pt_spawn_location (Variables|Default|GetPT_Spawn_Location))
  (bind _returnvalue (Transformation|GetWorldTransform _pt_spawn_location))
  ;[1 1 1] enemy touch player
  (bind _asbp_player (Utilities|Casting|CastToBP_Player OtherActor)) ; did player do the touch?
  (Utilities|IsValid _asbp_player
    (:Is%20Valid
      (if (Variables|enemyvulnerable|GetbIsVulnerable?) ; am vulnerable?
        (Utilities|FlowControl|Sequence
          (:then_0
            ;[1 1 1] eaten score fx
            (Utilities|EnemyEatenPoints
              (:%20%201%20enemy%20eaten
                (Game|SpawnActorfromClass "/Game/ArcadeClassic/Blueprints/Misc/BP_Score_200.BP_Score_200_C" _returnvalue "Undefined" 0 0))
              (:2nd%20enemy%20eaten
                (Game|SpawnActorfromClass "/Game/ArcadeClassic/Blueprints/Misc/BP_Score_400.BP_Score_400_C" _returnvalue "Undefined" 0 0))
              (:3rd%20enemy%20eaten
                (Game|SpawnActorfromClass "/Game/ArcadeClassic/Blueprints/Misc/BP_Score_800.BP_Score_800_C" _returnvalue "Undefined" 0 0))
              (:4th%20enemy%20eaten
                (Game|SpawnActorfromClass "/Game/ArcadeClassic/Blueprints/Misc/BP_Score_1600.BP_Score_1600_C" _returnvalue "Undefined" 0 0))))
          (:then_1
            ;[1 1 1] enemy eaten respawn
            (CallFunction|CloseEnemyNavGate) ; stop just this enemy
            (CallFunction|EnemyEatenFX)
            (Collision|SetCollisionResponsetoChannel (Variables|Default|GetPlayer_collision) "ECC_Pawn" "ECR_Ignore")
            (Variables|enemyvulnerable|SetbIsVulnerable? false)
            (CallFunction|EnemyStateRegular)
            (Transformation|SetActorLocation (Variables|ChildParameters|GetEnemyRespawnLocation) false false)
            (Utilities|FlowControl|Delay 2.0)
            (Effects|SpawnEmitteratLocation "/Game/InfinityBladeEffects/Effects/FX_Monsters/FX_Monster_Deaths/P_Monster_Death_Large.P_Monster_Death_Large" (Variables|ChildParameters|GetEnemyRespawnLocation)) ; enemy respawn fx
            (Collision|SetCollisionResponsetoChannel (Variables|Default|GetPlayer_collision) "ECC_Pawn" "ECR_Overlap")
            (Utilities|FlowControl|Delay 1.0)
            (Rendering|SetActorHiddenInGame false)
            ;[1 1 1] call enemy restart
            (CallFunction|SetEnemyRestartTime)))
        (else
          (Default|CallKilledPlayer)
          ;[1 1 1] stop all enemy navigation
          (CallFunction|CloseEnemyNavGate (Variables|References|GetEnemies)) ; stop all enemies
          ;[1 1 1] send enemies home
          (Utilities|FlowControl|Delay 2.5)
          (CallFunction|ResetEnemiestoHome (Variables|References|GetEnemies)))))))

(event Custom|Power%20Pellet%20Eaten
  ;[1 1 1] vulnerablility sequence
  (Variables|enemyvulnerable|SetbIsVulnerable? true)
  (Default|CallVulnerable) ; calls event in game mode bp to change music
  (Variables|ChildParameters|SetEnemyNavType "NewEnumerator0")
  (CallFunction|PickNewNavPoint)
  (Timeline|Vulnerablility%20Sequence PlayFromStart
    (:Finished
      (CallFunction|EnemyStateRegular)
      (Variables|enemyvulnerable|SetbIsVulnerable? false)
      (if (Variables|ChildParameters|GetbIsHunterEnemy?)
        (Variables|ChildParameters|SetEnemyNavType "NewEnumerator1")
        (else
          (Variables|ChildParameters|SetEnemyNavType "NewEnumerator0")))
      (Default|CallNotVulnerable)
      ;[1 1 1] reset enemy point values
      (CallFunction|ResetEnemyPointValue))
    (:Start%20Phase%20#1
      (CallFunction|EnemyStateVulnerable01))
    (:Start%20Phase%20#2
      (if (Variables|enemyvulnerable|GetbIsVulnerable?)
        (CallFunction|EnemyStateVulnerable02)))))

(event Custom|reset%20enemies%20to%20home
  ;[1 1 1] enemies reset to home
  (CallFunction|EnemySpawnOutFX)
  ;[1 1 1] enemy eaten respawn
  (Transformation|SetActorLocation (Variables|ChildParameters|GetEnemyRespawnLocation) false false)
  (Utilities|FlowControl|Delay 2.0)
  (Effects|SpawnEmitteratLocation "/Game/InfinityBladeEffects/Effects/FX_Monsters/FX_Monster_Deaths/P_Monster_Death_Large.P_Monster_Death_Large" (Variables|ChildParameters|GetEnemyRespawnLocation)) ; enemy respawn fx
  (Collision|SetCollisionResponsetoChannel (Variables|Default|GetPlayer_collision) "ECC_Pawn" "ECR_Overlap")
  (Utilities|FlowControl|Delay 1.0)
  (Rendering|SetActorHiddenInGame false)
  ;[1 1 1] call enemy restart
  (CallFunction|SetEnemyRestartTime))

(event Custom|Set%20Enemy%20Start%20Time
  ;[1 1 1] Start Enemy Nav
  (Utilities|Time|SetTimerbyEvent (delegate Custom|Start%20Nav) (Variables|ChildParameters|GetEnemyStartTime)))

(event Custom|Start%20Nav
  ;[1 1 1] Start Enemy Nav
  (if (Variables|/Game/ArcadeClassic/Blueprints/Characters/BP_Player.BP_Player_C|GetbShouldPlayerGobble? (Variables|References|GetPlayer))
    (Components|Activation|Activate (Variables|Character|GetCharacterMovement) false)
    (Variables|Navigation|SetbAssignedTargetPoint false)
    (Utilities|FlowControl|Gate true) ; enters at Open
    (else
      (Utilities|Time|SetTimerbyEvent (delegate Custom|Start%20Nav) (Variables|ChildParameters|GetEnemyStartTime)))))

(event Custom|Pick%20New%20Nav%20Point
  ;[1 1 1] pick new nav point
  (Utilities|FlowControl|Delay 0.1)
  (Variables|Navigation|SetbAssignedTargetPoint false)
  (Utilities|FlowControl|Gate true) ; enters at Open
)

(event Custom|Close%20Enemy%20Nav%20Gate
  ;[1 1 1] stop enemy nav on player death
  (Components|Activation|Deactivate (Variables|Character|GetCharacterMovement))
  (Utilities|FlowControl|Gate true) ; enters at Close
)

(event Custom|Set%20Enemy%20RestartTime
  ;[1 1 1] restart enemy nav after enemy sent to house
  (Utilities|Time|SetTimerbyEvent (delegate Custom|Restart%20nav) (Variables|ChildParameters|GetEnemyRestartTime)))

(event Custom|Restart%20nav
  ;[1 1 1] restart enemy nav after enemy sent to house
  (if (Variables|/Game/ArcadeClassic/Blueprints/Characters/BP_Player.BP_Player_C|GetbShouldPlayerGobble? (Variables|References|GetPlayer))
    (Components|Activation|Activate (Variables|Character|GetCharacterMovement) false)
    (Variables|Navigation|SetbAssignedTargetPoint false)
    (Utilities|FlowControl|Gate true) ; enters at Open
    (else
      (Utilities|Time|SetTimerbyEvent (delegate Custom|Restart%20nav) (Variables|ChildParameters|GetEnemyRestartTime)))))

(event EventBeginPlay
  (Utilities|FlowControl|Sequence
    (:then_0
      ;[1 1 1] refrence to game instance
      (bind _asbp_game_instance (Utilities|Casting|CastToBP_GameInstance (Game|GetGameInstance)))
      (Variables|Default|SetGame%20Instance _asbp_game_instance)
      ;[1 1 1] reference to all enemies
      (bind _outactors (Actor|GetAllActorsOfClass "BP_Enemy_parent_C"))
      (Variables|References|SetEnemies _outactors)
      ;[1 1 1] reference to player
      (bind _asbp_player (Utilities|Casting|CastToBP_Player (Game|GetPlayerCharacter 0)))
      (Variables|References|SetPlayer _asbp_player)
      ;[1 1 1] reference to target points
      (bind _outactors_2 (Actor|GetAllActorsOfClass "/Script/Engine.TargetPoint"))
      (Variables|References|SetTarget%20Point _outactors_2)
      ;[1 1 1] stores enemies spawn locations
      (Variables|ChildParameters|SetEnemyRespawnLocation (Transformation|GetActorLocation)))
    (:then_1
      ;[1 1 1] opens gate for enemy nav
      (CallFunction|SetEnemyStartTime))))

(event EventTick
  (params (DeltaSeconds :type Float%20%28single-precision%29))
  (Utilities|FlowControl|Gate true
    (:Exit
      (switch Utilities|FlowControl|Switch|SwitchonEnemyNavTypes (Variables|ChildParameters|GetEnemyNavType)
        (:NewEnumerator0
          (if (Variables|Navigation|GetbAssignedTargetPoint)
            ;[1 1 1] target got to target point? then pick new location
            (if (<= (Transformation|GetDistanceTo (Variables|Navigation|GetEnemySelectedTarget)) (Variables|ChildParameters|GetEnemyTargetAcceptanceRadius))
              (CallFunction|PickNewNavPoint))
            (else
              ;[1 1 1] wandering enemy nav
              (CallFunction|NavigationWander))))
        (:NewEnumerator1
          ;[1 1 1] hunter enemy nav
          (CallFunction|NavigationHunter))))))

(fn ConstructionScript)

(fn EnemyStateRegular
  (Rendering|SetVisibility (Variables|Default|GetEnemy_Vulnerable_01) false false)
  (Rendering|SetVisibility (Variables|Default|GetEnemy_Down) true false))

(fn EnemyStateVulnerable01
  (Rendering|SetVisibility (Variables|Default|GetEnemy_Vulnerable_02) false false)
  (Rendering|SetVisibility (Variables|Default|GetEnemy_Vulnerable_01) true false))

(fn EnemyStateVulnerable02
  (Rendering|SetVisibility (Variables|Default|GetEnemy_Down) false false)
  (Rendering|SetVisibility (Variables|Default|GetEnemy_Vulnerable_02) true false))

(fn EnemyEatenFX
  (Effects|SpawnEmitteratLocation "/Game/ArcadeClassic/Particles/P_Death.P_Death" (Transformation|GetWorldLocation (Variables|Collision|GetCapsuleComponent)))
  (Audio|PlaySound2D "/Game/ArcadeClassic/Audio/SFX_EatEnemy_Cue.SFX_EatEnemy_Cue" 1.0 1.0 0.0 0 0)
  (Rendering|SetActorHiddenInGame true))

(fn EnemySpawnOutFX
  (Effects|SpawnEmitteratLocation "/Game/ArcadeClassic/Particles/P_SpawnOut_enemy.P_SpawnOut_enemy" (Transformation|GetWorldLocation (Variables|Collision|GetCapsuleComponent))) ; spawn out vfx
  (Rendering|SetActorHiddenInGame true))

(fn NavigationWander
  (bind _target_point (Variables|References|GetTarget%20Point))
  (bind _output_get (Variables|Navigation|SetEnemySelectedTarget (Utilities|Array|Get(acopy) _target_point (Math|Random|RandomInteger (Utilities|Array|Length _target_point)))))
  (AI|Navigation|MovetoLocation (AI|GetAIController (Pawn|GetController)) (Transformation|GetActorLocation _output_get) -1.0 true true false true 0)
  (Variables|Navigation|SetbAssignedTargetPoint true))

(fn NavigationHunter
  (AI|Navigation|MovetoLocation (AI|GetAIController (Pawn|GetController)) (Transformation|GetWorldLocation (Variables|/Script/Engine.Character|GetCapsuleComponent (Variables|References|GetPlayer))) -1.0 true true false true 0))

(fn ResetEnemyPointValue
  (bind _player (Variables|References|GetPlayer))
  (Variables|/Game/ArcadeClassic/Blueprints/Characters/BP_Player.BP_Player_C|SetbHaveEaten1Enemy? _player false)
  (Variables|/Game/ArcadeClassic/Blueprints/Characters/BP_Player.BP_Player_C|SetbHaveEaten2Enemy? _player false)
  (Variables|/Game/ArcadeClassic/Blueprints/Characters/BP_Player.BP_Player_C|SetbHaveEaten3Enemy? _player false)
  (Variables|/Game/ArcadeClassic/Blueprints/Characters/BP_Player.BP_Player_C|SetbHaveEaten4Enemy? _player false))